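; Map editor gizmo that scales its RelatedActor along X, Y or Z through colored, hover-highlighted handles.
; Clicking a handle picks the axis and saves the scale; mouse movement is projected onto that axis relative to the pawn's view direction until release.
; Ctrl+Z and Ctrl+Y step through saved scales in undo and repeat arrays.
; UpdateSensitivity runs on Tick but is empty, with its distance-based sensitivity and gizmo sizing disconnected.
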(event `self.DeActivate`
  (bind _relatedactor (`self.RelatedActor`))
  (`|ExecutionSequence`
    (:`then_0`
      (`/Engine/EditorBlueprintResources/StandardMacros.IsValid` (`self.RelatedActor`)
        (:`Is Valid`
          (`self.SetActorEnableCollision` _relatedactor true)
          (`self.SetActorHiddenInGame` _relatedactor false))))
    (:`then_1`
      (`parent.DeActivate`))))

(event `self.Activate`
  (bind _relatedactor (`self.RelatedActor`))
  (`parent.Activate`)
  (`self.SetActorEnableCollision` _relatedactor false)
  (`self.SetActorRotation` (`self.K2_GetActorRotation` _relatedactor)))

(event `Key|Ctrl+Z`
  (bind _undoarray (`self.UndoArray`))
  (bind _relatedactor (`self.RelatedActor`))
  (bind _returnvalue (`KismetArrayLibrary.Array_LastIndex` _undoarray))
  (bind _item (`KismetArrayLibrary.Array_Get` _undoarray _returnvalue))
  ;[1 1 1] Repeat/Undo
  (:`Pressed`
    (if (< (`self.MoveDirection`) 0)
      (if (> (`KismetArrayLibrary.Array_Length` (`self.UndoArray`)) 0)
        (`/Engine/EditorBlueprintResources/StandardMacros.IsValid` _relatedactor
          (:`Is Valid`
            (`self.SetActorScale3D` _relatedactor _item)
            (`KismetArrayLibrary.Array_Add` (`self.RepeatArray`) _item)
            (`KismetArrayLibrary.Array_Remove` (`self.UndoArray`) _returnvalue)))))))

(event `Key|LeftMouseButton`
  (:`Released`
    (set `self.MoveDirection` -1) ; Disable movement
  ))

(event `self.ReceiveActorBeginOverlap`
  (params (OtherActor :type "Actor Object Reference")))

(event `Key|Ctrl+Y`
  (bind _repeatarray (`self.RepeatArray`))
  (bind _relatedactor (`self.RelatedActor`))
  (bind _returnvalue (`KismetArrayLibrary.Array_LastIndex` _repeatarray))
  (bind _item (`KismetArrayLibrary.Array_Get` _repeatarray _returnvalue))
  ;[1 1 1] Repeat/Undo
  (:`Pressed`
    (if (< (`self.MoveDirection`) 0)
      (if (> (`KismetArrayLibrary.Array_Length` (`self.RepeatArray`)) 0)
        (`/Engine/EditorBlueprintResources/StandardMacros.IsValid` _relatedactor
          (:`Is Valid`
            (`self.SetActorScale3D` _relatedactor _item)
            (`KismetArrayLibrary.Array_Add` (`self.UndoArray`) _item)
            (`KismetArrayLibrary.Array_Remove` (`self.RepeatArray`) _returnvalue)))))))

(event `self.ReceiveTick`
  (params (DeltaSeconds :type "Float (single-precision)"))
  (`self.UpdateSensitivity`)
  (`/Engine/EditorBlueprintResources/StandardMacros.IsValid` (`self.RelatedActor`)))

(event `InputAxisKey|MouseX`
  (params (AxisValue :type "Float (single-precision)"))
  (`self.ScaleRelatedActor` AxisValue (stale `InputAxisKey|MouseY` AxisValue) :!label _label))

(event `InputAxisKey|MouseY`
  (params (AxisValue :type "Float (single-precision)"))
  (goto _label))

(event `self.Direction_X.OnClicked`
  (params (TouchedComponent :type "PrimitiveComponent Object Reference"))
  (bind _relatedactor (`self.RelatedActor`))
  ;[1 1 1] Movement modes
  (set `self.MoveDirection` 0)
  (`self.EnableInput` (`self.OwnerPC`) :!label _label_2)
  (`/Engine/EditorBlueprintResources/StandardMacros.IsValid` _relatedactor
    (:`Is Valid`
      (`KismetArrayLibrary.Array_Add` (`self.UndoArray`) (`self.GetActorScale3D` _relatedactor)))))

(event `self.Direction_Y.OnClicked`
  (params (TouchedComponent :type "PrimitiveComponent Object Reference"))
  ;[1 1 1] Movement modes
  (set `self.MoveDirection` 1)
  (goto _label_2))

(event `self.Direction_Z.OnClicked`
  (params (TouchedComponent :type "PrimitiveComponent Object Reference"))
  ;[1 1 1] Movement modes
  (set `self.MoveDirection` 2)
  (goto _label_2))

(event `self.Direction_Z.OnBeginCursorOver`
  (params (TouchedComponent :type "PrimitiveComponent Object Reference"))
  ;[1 1 1] Cursor Hovering
  (`MaterialInstanceDynamic.SetVectorParameterValue` (`self.MID_Z`) "Color" (struct :`R` 255.0 :`G` 255.0 :`A` 1.0)))

(event `self.Direction_Z.OnEndCursorOver`
  (params (TouchedComponent :type "PrimitiveComponent Object Reference"))
  ;[1 1 1] Cursor Hovering
  (`MaterialInstanceDynamic.SetVectorParameterValue` (`self.MID_Z`) "Color" (struct :`B` 255.0 :`A` 1.0)))

(event `self.Direction_Y.OnBeginCursorOver`
  (params (TouchedComponent :type "PrimitiveComponent Object Reference"))
  ;[1 1 1] Cursor Hovering
  (`MaterialInstanceDynamic.SetVectorParameterValue` (`self.MID_Y`) "Color" (struct :`R` 255.0 :`G` 255.0 :`A` 1.0)))

(event `self.Direction_Y.OnEndCursorOver`
  (params (TouchedComponent :type "PrimitiveComponent Object Reference"))
  ;[1 1 1] Cursor Hovering
  (`MaterialInstanceDynamic.SetVectorParameterValue` (`self.MID_Y`) "Color" (struct :`G` 255.0 :`A` 1.0)))

(event `self.Direction_X.OnBeginCursorOver`
  (params (TouchedComponent :type "PrimitiveComponent Object Reference"))
  ;[1 1 1] Cursor Hovering
  (`MaterialInstanceDynamic.SetVectorParameterValue` (`self.MID_X`) "Color" (struct :`R` 255.0 :`G` 255.0 :`A` 1.0)))

(event `self.Direction_X.OnEndCursorOver`
  (params (TouchedComponent :type "PrimitiveComponent Object Reference"))
  ;[1 1 1] Cursor Hovering
  (`MaterialInstanceDynamic.SetVectorParameterValue` (`self.MID_X`) "Color" (struct :`R` 255.0 :`A` 1.0)))

(fn `ScaleRelatedActor`
  (params (X :type "Float (double-precision)" :default 0.0) (Y :type "Float (double-precision)" :default 0.0))
  (bind _returnvalue (`self.K2_GetActorRotation`))
  (bind _relatedactor (`self.RelatedActor`))
  (bind _sensitivity (`self.Sensitivity`))
  (bind _sensitivity_2 (`self.Sensitivity`))
  (bind _relatedactor_2 (`self.RelatedActor`))
  (bind _relatedactor_3 (`self.RelatedActor`))
  (bind _sensitivity_3 (`self.Sensitivity`))
  (bind _returnvalue_2 (`KismetMathLibrary.MakeRot` 0.0 (.yaw _returnvalue)))
  (bind (_x _y) (`KismetMathLibrary.BreakRotIntoAxes` _returnvalue_2))
  (bind _returnvalue_3 (`KismetMathLibrary.FindLookAtRotation` (`self.K2_GetActorLocation` (`Controller.K2_GetPawn` (`self.OwnerPC`))) (`self.K2_GetActorLocation`)))
  (bind _x_2 (`KismetMathLibrary.BreakRotIntoAxes` _returnvalue_2))
  (bind _returnvalue_4 (`KismetMathLibrary.Dot_VectorVector` (`.Z` (`KismetMathLibrary.BreakRotIntoAxes` _returnvalue)) (`.Z` (`KismetMathLibrary.BreakRotIntoAxes` _returnvalue_3))))
  (bind _returnvalue_5 (`KismetMathLibrary.MakeRot` 0.0 (.yaw _returnvalue_3)))
  (bind (_x_3 _y_2) (`KismetMathLibrary.BreakRotIntoAxes` _returnvalue_5))
  (bind (_x_4 _y_3) (`KismetMathLibrary.BreakRotIntoAxes` _returnvalue_5))
  (switch `int` (`self.MoveDirection`)
    (:`0`
      (`self.SetActorScale3D` _relatedactor_2 (`KismetMathLibrary.MakeVector` (+ (.x (`self.GetActorScale3D` _relatedactor_2)) (/ (+ (* X (`KismetMathLibrary.Dot_VectorVector` _x_2 _y_3) _sensitivity) (* Y (`KismetMathLibrary.Dot_VectorVector` _x_2 _x_4) _sensitivity)) 100.0)) (.y (`self.GetActorScale3D` _relatedactor_2)) (.z (`self.GetActorScale3D` _relatedactor_2)))))
    (:`1`
      (`self.SetActorScale3D` _relatedactor_3 (`KismetMathLibrary.MakeVector` (.x (`self.GetActorScale3D` _relatedactor_3)) (+ (.y (`self.GetActorScale3D` _relatedactor_3)) (/ (+ (* X (`KismetMathLibrary.Dot_VectorVector` _y _y_2) _sensitivity_2) (* Y (`KismetMathLibrary.Dot_VectorVector` _x_3 _y) _sensitivity_2)) 100.0)) (.z (`self.GetActorScale3D` _relatedactor_3)))))
    (:`2`
      (`self.SetActorScale3D` _relatedactor (`KismetMathLibrary.MakeVector` (.x (`self.GetActorScale3D` _relatedactor)) (.y (`self.GetActorScale3D` _relatedactor)) (+ (.z (`self.GetActorScale3D` _relatedactor)) (/ (+ (* (* -1 X) _returnvalue_4 _sensitivity_3) (* Y _returnvalue_4 _sensitivity_3)) 100.0)))))))

(fn `UpdateSensitivity`)

(fn `UserConstructionScript`
  (`parent.UserConstructionScript`)
  (`|ExecutionSequence`
    (:`then_0`
      (bind _returnvalue (`KismetMaterialLibrary.CreateDynamicMaterialInstance` "/Game/MapEditorExample/Materials/M_Color.M_Color"))
      (bind _output_get (set `self.MID_X` _returnvalue))
      (`PrimitiveComponent.SetMaterial` (`self.Direction_X`) 0 _output_get)
      (`MaterialInstanceDynamic.SetVectorParameterValue` (`self.MID_X`) "Color" (struct :`R` 255.0 :`A` 1.0)))
    (:`then_1`
      (bind _returnvalue_2 (`KismetMaterialLibrary.CreateDynamicMaterialInstance` "/Game/MapEditorExample/Materials/M_Color.M_Color"))
      (bind _output_get_2 (set `self.MID_Y` _returnvalue_2))
      (`PrimitiveComponent.SetMaterial` (`self.Direction_Y`) 0 _output_get_2)
      (`MaterialInstanceDynamic.SetVectorParameterValue` (`self.MID_Y`) "Color" (struct :`G` 255.0 :`A` 1.0)))
    (:`then_2`
      (bind _returnvalue_3 (`KismetMaterialLibrary.CreateDynamicMaterialInstance` "/Game/MapEditorExample/Materials/M_Color.M_Color"))
      (bind _output_get_3 (set `self.MID_Z` _returnvalue_3))
      (`PrimitiveComponent.SetMaterial` (`self.Direction_Z`) 0 _output_get_3)
      (`MaterialInstanceDynamic.SetVectorParameterValue` (`self.MID_Z`) "Color" (struct :`B` 255.0 :`A` 1.0)))))