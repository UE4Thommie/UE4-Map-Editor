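; Map editor controller that traces under the cursor each tick to select actors and hand them to transform modifiers.
; Selection accepts saveable or static mesh actors, and pulls clicked instanced-mesh instances out through SaveGame_Manager as actors.
; A new selection rebuilds the modifier list and activates the default; only the move modifier is spawned so far.
; Left click fires a rebindable dispatcher, which activating a modifier clears.
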(event `DefaultBindings`
  (`|ExecutionSequence`
    (:`then_0`
      (clear `self.OnLMBPressed`)
      (add `self.OnLMBPressed` (`|CreateDelegate` self :!event `SelectActor`)))))

(event `self.ReceiveBeginPlay`
  (`self.DefaultBindings`)
  (bind _returnvalue (`|SpawnActorFromClass` "/Game/MapEditorExample/Blueprints/Modifiers/BP_ModifyActor_Location.BP_ModifyActor_Location_C" (`KismetMathLibrary.MakeTransform` (0.0 0.0 0.0))))
  (set `self.MOD_MoveActor` _returnvalue))

(event `self.ReceiveTick`
  (params (DeltaSeconds :type "Float (single-precision)"))
  (bind _hitresult (`self.GetHitResultUnderCursorByChannel` "TraceTypeQuery1"))
  (set `self.CursorHitActor` (`.HitActor` (`GameplayStatics.BreakHitResult` _hitresult)))
  (set `self.CursorHitLocation` (`.ImpactPoint` (`GameplayStatics.BreakHitResult` _hitresult)))
  (set `self.CursorHitComponent` (`.HitComponent` (`GameplayStatics.BreakHitResult` _hitresult))))

(event `Key|LeftMouseButton`
  (:`Pressed`
    (`self.OnLMBPressed`)))

(fn `BuildModifierList`
  (params (ModifierClasses :type "Array of /Game/MapEditorExample/Blueprints/Modifiers/BP_ModifyActor_Base Class Reference"))
  (`|ExecutionSequence`
    (:`then_0`
      (`KismetArrayLibrary.Array_RemoveItem` (`self.ModifierList`) (`self.MOD_MoveActor`))
      (`KismetArrayLibrary.Array_RemoveItem` (`self.ModifierList`) (`self.MOD_RotateActor`))
      (`KismetArrayLibrary.Array_RemoveItem` (`self.ModifierList`) (`self.MOD_ScaleActor`)))
    (:`then_1`
      (for _array_element (`self.ModifierList`)
        (`self.K2_DestroyActor` _array_element))
      (`KismetArrayLibrary.Array_Clear` (`self.ModifierList`)))
    (:`then_2`
      (`KismetArrayLibrary.Array_Add` (`self.ModifierList`) (`self.MOD_MoveActor`))
      (`KismetArrayLibrary.Array_Add` (`self.ModifierList`) (`self.MOD_RotateActor`))
      (`KismetArrayLibrary.Array_Add` (`self.ModifierList`) (`self.MOD_ScaleActor`)))
    (:`then_3`
      (for _array_element_2 ModifierClasses
        (bind _returnvalue (`|SpawnActorFromClass` _array_element_2 (`KismetMathLibrary.MakeTransform` (0.0 0.0 0.0)) true))
        (`KismetArrayLibrary.Array_AddUnique` (`self.ModifierList`) _returnvalue)))
    (:`then_4`
      (for _array_element_3 (`self.ModifierList`)
        (if (== (`GameplayStatics.GetObjectClass` _array_element_3) (`self.DefaultModifierClass`))
          (`self.SetActiveModifier` _array_element_3 (`self.SelectedActor`))
          (break))))))

(fn `SelectActor`
  (bind _asinstanced_static_mesh_component (cast `InstancedStaticMeshComponent` (`self.CursorHitComponent`) :!pure true))
  (bind _assave_game_manager (cast `/Game/MapEditorExample/Blueprints/Saving/SaveGame_Manager` (`self.CursorHitActor`))
    (:`then`
      (bind _instanceindex (`/Game/MapEditorExample/Blueprints/Saving/SaveGame_Manager.GetInstanceIndex` _assave_game_manager _asinstanced_static_mesh_component (`self.CursorHitLocation`)))
      (if (> _instanceindex -1)
        (bind _newactor (`/Game/MapEditorExample/Blueprints/Saving/SaveGame_Manager.RemoveInstance` _assave_game_manager _asinstanced_static_mesh_component _instanceindex false))
        (`self.SelectNewActor` _newactor)))
    (:`CastFailed`
      (if (`KismetSystemLibrary.DoesImplementInterface` (`self.CursorHitActor`) "/Game/MapEditorExample/Blueprints/Saving/I_SaveableActor.I_SaveableActor_C")
        (`self.SelectNewActor` (`self.CursorHitActor`))
        (else
          (bind _asbp_static_mesh_actor (cast `/Game/MapEditorExample/Blueprints/Saving/BP_StaticMeshActor` (`self.CursorHitActor`))
            (:`then`
              (`self.SelectNewActor` _asbp_static_mesh_actor))
            (:`CastFailed`
              (`self.SelectNewActor` null))))))))

(fn `SelectNewActor`
  (params (NewActor :type "Actor Object Reference"))
  (`/Engine/EditorBlueprintResources/StandardMacros.IsValid` NewActor
    (:`Is Valid`
      (`/Engine/EditorBlueprintResources/StandardMacros.IsValid` (`self.SelectedActor`)
        (:`Is Valid`
          (if (!= (`self.SelectedActor`) NewActor)
            (set `self.SelectedActor` null)
            (set `self.SelectedActor` NewActor :!label _label)
            (`self.BuildModifierList` (`|MakeArray` null :!type "/Game/MapEditorExample/Blueprints/Modifiers/BP_ModifyActor_Base Class Reference"))))
        (:`Is Not Valid`
          (goto _label))))
    (:`Is Not Valid`
      ;[1 1 1] @TODO Deselect Selected Actor
      (set `self.SelectedActor` null))))

(fn `SetActiveModifier`
  (params (NewModifier :type "/Game/MapEditorExample/Blueprints/Modifiers/BP_ModifyActor_Base Object Reference") (ForActor :type "Actor Object Reference"))
  (`/Engine/EditorBlueprintResources/StandardMacros.IsValid` ForActor
    (:`Is Valid`
      (`/Engine/EditorBlueprintResources/StandardMacros.IsValid` NewModifier
        (:`Is Valid`
          (`/Engine/EditorBlueprintResources/StandardMacros.IsValid` (`self.ActiveModifier`)
            (:`Is Valid`
              (`/Game/MapEditorExample/Blueprints/Modifiers/BP_ModifyActor_Base.DeActivate` (`self.ActiveModifier`)))
            (:`Is Not Valid`
              _))
          (bind _output_get (set `self.ActiveModifier` NewModifier))
          (`/Game/MapEditorExample/Blueprints/Modifiers/BP_ModifyActor_Base.Activate` _output_get ForActor)
          (clear `self.OnLMBPressed`))
        (:`Is Not Valid`
          (`/Engine/EditorBlueprintResources/StandardMacros.IsValid` (`self.ActiveModifier`)
            (:`Is Valid`
              (`/Game/MapEditorExample/Blueprints/Modifiers/BP_ModifyActor_Base.DeActivate` (`self.ActiveModifier`))
              (set `self.ActiveModifier` null)
              ;[1 1 1] Reset LMB binding to default
              (clear `self.OnLMBPressed`)
              (add `self.OnLMBPressed` (`|CreateDelegate` self :!event `SelectActor`)))))))))

(fn `UserConstructionScript`)