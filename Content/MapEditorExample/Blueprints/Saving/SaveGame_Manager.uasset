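; Map editor manager actor that places static meshes, saves and loads levels, and tracks save slots in a persistent SaveFileList.
; New meshes spawn as actors; the oldest beyond a limit become capped-size instanced mesh components, and removed instances can become actors again.
; Saving converts remaining recent actors to instances, then stores per-mesh transforms plus data from I_SaveableActor actors.
; Loading clears the level and rebuilds both.
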(event Custom|GetSaveFileList
  (bind _returnvalue (SaveGame|DoesSaveGameExist "SaveFileList"))
  (if _returnvalue
    (bind _returnvalue_2 (SaveGame|LoadGamefromSlot "SaveFileList"))
    (bind _assave_file_list (Utilities|Casting|CastToSaveFileList _returnvalue_2))
    (for _array_element (Variables|/Game/MapEditorExample/Blueprints/Saving/SaveFileList.SaveFileList_C|GetSaveFiles _assave_file_list)
      (bind _returnvalue_3 (SaveGame|DoesSaveGameExist (.FileName (Utilities|Struct|BreakSTRUCT_SaveFileInfo _array_element)) (.Index (Utilities|Struct|BreakSTRUCT_SaveFileInfo _array_element))))
      (if _returnvalue_3
        (Utilities|Array|Add (Variables|Default|GetSaveFiles) _array_element)))))

(event Custom|CreateSaveFileList
  (bind _returnvalue (SaveGame|CreateSaveGameObject "/Game/MapEditorExample/Blueprints/Saving/SaveFileList.SaveFileList_C"))
  (bind _assave_file_list (Utilities|Casting|CastToSaveFileList _returnvalue))
  (Variables|/Game/MapEditorExample/Blueprints/Saving/SaveFileList.SaveFileList_C|SetSaveFiles _assave_file_list (Variables|Default|GetSaveFiles))
  (SaveGame|SaveGametoSlot _assave_file_list "SaveFileList"))

(event Custom|CheckRecentISMS
  (bind _recentsmactors (Variables|Level|GetRecentSMActors))
  (bind _item (Utilities|Array|Get(acopy) _recentsmactors))
  (while (> (Utilities|Array|Length (Variables|Level|GetRecentSMActors)) (Variables|Default|GetMaxRecentSMActorsLength))
    (CallFunction|AddArrayISM (Variables|/Script/Engine.StaticMeshComponent|GetStaticMesh (Variables|/Game/MapEditorExample/Blueprints/Saving/BP_StaticMeshActor.BP_StaticMeshActor_C|GetStaticMesh _item)) (Transformation|GetActorTransform _item))
    (Actor|DestroyActor _item)
    (Utilities|Array|RemoveItem (Variables|Level|GetRecentSMActors) _item)))

(event Custom|ClearLevel
  (Utilities|FlowControl|Sequence
    (:then_0
      (bind _outactors (Actor|GetAllActorswithInterface "/Game/MapEditorExample/Blueprints/Saving/I_SaveableActor.I_SaveableActor_C"))
      (for _array_element _outactors
        (Actor|DestroyActor _array_element)))
    (:then_1
      (for _array_element_2 (Variables|Level|GetISM_Components)
        (Components|DestroyComponent _array_element_2))
      (Utilities|Array|Clear (Variables|Level|GetISM_Components)))
    (:then_2
      (for _array_element_3 (Variables|Level|GetRecentSMActors)
        (Actor|DestroyActor _array_element_3))
      (Utilities|Array|Clear (Variables|Level|GetRecentSMActors)))))

(event Custom|RemoveSaveFile
  (params (Slot%20Name :type String) (Index :type Integer :default 0))
  (bind _array_element (Utilities|Array|ForEachLoopwithBreak (Variables|Default|GetSaveFiles))
    (:LoopBody
      (if (and (Utilities|Enum|Equal(Enum) (.FileName (Utilities|Struct|BreakSTRUCT_SaveFileInfo _array_element)) Slot%20Name) (== (.Index (Utilities|Struct|BreakSTRUCT_SaveFileInfo _array_element)) Index))
        (SaveGame|DeleteGameinSlot (.FileName (Utilities|Struct|BreakSTRUCT_SaveFileInfo _array_element)) (.Index (Utilities|Struct|BreakSTRUCT_SaveFileInfo _array_element)))
        (Utilities|Array|RemoveItem (Variables|Default|GetSaveFiles) _array_element)))
    (:Completed
      (CallFunction|CreateSaveFileList))))

(event EventDestroyed
  (CallFunction|CreateSaveFileList))

(event EventBeginPlay
  (CallFunction|GetSaveFileList))

(event EventActorBeginOverlap
  (params (OtherActor :type Actor%20Object%20Reference)))

(event EventTick
  (params (DeltaSeconds :type Float%20%28single-precision%29)))

(fn ConstructionScript)

(fn AddArrayISM
  (params (Mesh :type Static%20Mesh%20Object%20Reference) (Transform :type Transform))
  (bind _array_element (Utilities|Array|ForEachLoopwithBreak (Variables|Level|GetISM_Components) :!label _label)
    (:LoopBody
      (if (== (Variables|/Script/Engine.StaticMeshComponent|GetStaticMesh _array_element) Mesh)
        (if (>= (Components|InstancedStaticMesh|GetInstanceCount _array_element) (Variables|Default|GetMaxISMArrayLength))
          (LocalVariables|SetbAddNew true)
          (else
            (LocalVariables|SetbAddNew false)
            (Class|InstancedStaticMeshComponent|AddInstanceWorldSpace _array_element Transform)
            (goto _label Break)))
        (else
          (LocalVariables|SetbAddNew true))))
    (:Completed
      (if (LocalVariables|GetbAddNew)
        (CallFunction|AddISMComponent Mesh Transform)))))

(fn AddStaticMesh
  (params (Mesh :type Static%20Mesh%20Object%20Reference) (Transform :type Transform))
  (bind _returnvalue (Game|SpawnActorfromClass "/Game/MapEditorExample/Blueprints/Saving/BP_StaticMeshActor.BP_StaticMeshActor_C" Transform true 0))
  (Utilities|Array|Add (Variables|Level|GetRecentSMActors) _returnvalue)
  (Components|StaticMesh|SetStaticMesh (Variables|/Game/MapEditorExample/Blueprints/Saving/BP_StaticMeshActor.BP_StaticMeshActor_C|GetStaticMesh _returnvalue) Mesh)
  (CallFunction|CheckRecentISMS)
  (return _returnvalue))

(fn AddISMComponent
  (params (Mesh :type Static%20Mesh%20Object%20Reference) (Transform :type Transform))
  (bind _returnvalue (AddComponent|AddInstancedStaticMeshComponent false))
  (Utilities|Array|Add (Variables|Level|GetISM_Components) _returnvalue)
  (Components|StaticMesh|SetStaticMesh _returnvalue Mesh)
  (Class|InstancedStaticMeshComponent|AddInstanceWorldSpace _returnvalue Transform))

(fn GetInstanceIndex
  (params (Component :type Instanced%20Static%20Mesh%20Component%20Object%20Reference) (HitLocation :type Vector :default "0, 0, 0"))
  (bind _index (Utilities|FlowControl|ForLoopwithBreak 0 (Components|InstancedStaticMesh|GetInstanceCount Component))
    (:LoopBody
      (if (.ReturnValue (Components|InstancedStaticMesh|GetInstanceTransform Component _index true))
        (if (< (Math|Vector|VectorLength (- (.Location (Math|Transform|BreakTransform (.OutInstanceTransform (Components|InstancedStaticMesh|GetInstanceTransform Component _index true)))) HitLocation)) (LocalVariables|GetDistance))
          (LocalVariables|SetDistance (Math|Vector|VectorLength (- (.Location (Math|Transform|BreakTransform (.OutInstanceTransform (Components|InstancedStaticMesh|GetInstanceTransform Component _index true)))) HitLocation)))
          (LocalVariables|SetIndex _index))))
    (:Completed
      (return (LocalVariables|GetIndex)))))

(fn RemoveInstance
  (params (Component :type Instanced%20Static%20Mesh%20Component%20Object%20Reference) (Index :type Integer :default 0) (bDestroy :type Boolean :default false))
  (if bDestroy
    (Class|InstancedStaticMeshComponent|RemoveInstance Component Index)
    (else
      (bind _newactor (CallFunction|AddStaticMesh (Variables|/Script/Engine.StaticMeshComponent|GetStaticMesh Component) (.OutInstanceTransform (Components|InstancedStaticMesh|GetInstanceTransform Component Index true))))
      (Class|InstancedStaticMeshComponent|RemoveInstance Component Index)
      (return _newactor))))

(fn SaveGame
  (params (Slot%20Name :type String) (Index :type Integer :default 0))
  (for _array_element (Variables|Level|GetRecentSMActors)
    (CallFunction|AddArrayISM (Variables|/Script/Engine.StaticMeshComponent|GetStaticMesh (Variables|/Game/MapEditorExample/Blueprints/Saving/BP_StaticMeshActor.BP_StaticMeshActor_C|GetStaticMesh _array_element)) (Transformation|GetActorTransform _array_element))
    (Actor|DestroyActor _array_element))
  (Utilities|Array|Clear (Variables|Level|GetRecentSMActors))
  (bind _returnvalue (SaveGame|CreateSaveGameObject "/Game/MapEditorExample/Blueprints/Saving/Editor_SaveGame.Editor_SaveGame_C"))
  (bind _aseditor_save_game (Utilities|Casting|CastToEditor_SaveGame _returnvalue))
  (LocalVariables|SetEditorSaveGame _aseditor_save_game)
  (Utilities|FlowControl|Sequence
    (:then_0
      (for _array_element_2 (Variables|Level|GetISM_Components)
        (for _index (range 0 (Components|InstancedStaticMesh|GetInstanceCount _array_element_2))
          (Utilities|Array|Add (LocalVariables|GetTransforms) (.OutInstanceTransform (Components|InstancedStaticMesh|GetInstanceTransform _array_element_2 _index true))))
        (Utilities|Array|Add (Variables|/Game/MapEditorExample/Blueprints/Saving/Editor_SaveGame.Editor_SaveGame_C|GetISMS (LocalVariables|GetEditorSaveGame)) (Utilities|Struct|MakeSTRUCT_ISM_Save (Variables|/Script/Engine.StaticMeshComponent|GetStaticMesh _array_element_2) (LocalVariables|GetTransforms)))
        (Utilities|Array|Clear (LocalVariables|GetTransforms))))
    (:then_1
      (bind _outactors (Actor|GetAllActorswithInterface "/Game/MapEditorExample/Blueprints/Saving/I_SaveableActor.I_SaveableActor_C"))
      (for _array_element_3 _outactors
        (bind _savestats (Class|ISaveableActor|GetSaveStats(Message) _array_element_3))
        (Utilities|Array|Add (Variables|/Game/MapEditorExample/Blueprints/Saving/Editor_SaveGame.Editor_SaveGame_C|GetActors (LocalVariables|GetEditorSaveGame)) _savestats)))
    (:then_2
      (bind _returnvalue_2 (SaveGame|SaveGametoSlot (LocalVariables|GetEditorSaveGame) Slot%20Name Index))
      (if _returnvalue_2
        (bind _array_element_4 (Utilities|Array|ForEachLoopwithBreak (Variables|Default|GetSaveFiles) :!label _label)
          (:LoopBody
            (if (and (Utilities|Enum|Equal(Enum) (.FileName (Utilities|Struct|BreakSTRUCT_SaveFileInfo _array_element_4)) Slot%20Name) (== (.Index (Utilities|Struct|BreakSTRUCT_SaveFileInfo _array_element_4)) Index))
              (LocalVariables|SetbSaveOverwritten true)
              (goto _label Break)))
          (:Completed
            (if (not (LocalVariables|GetbSaveOverwritten))
              (Utilities|Array|Add (Variables|Default|GetSaveFiles) (Utilities|Struct|MakeSTRUCT_SaveFileInfo Slot%20Name Index))
              (CallFunction|CreateSaveFileList))))))))

(fn LoadGame
  (params (Slot%20Name :type String) (Index :type Integer :default 0))
  (bind _returnvalue (SaveGame|DoesSaveGameExist Slot%20Name Index))
  (if _returnvalue
    (bind _returnvalue_2 (SaveGame|LoadGamefromSlot Slot%20Name Index))
    (bind _aseditor_save_game (Utilities|Casting|CastToEditor_SaveGame _returnvalue_2))
    (LocalVariables|SetEditorSaveGame _aseditor_save_game)
    (CallFunction|ClearLevel)
    (Utilities|FlowControl|Sequence
      (:then_0
        (for _array_element (Variables|/Game/MapEditorExample/Blueprints/Saving/Editor_SaveGame.Editor_SaveGame_C|GetISMS (LocalVariables|GetEditorSaveGame))
          (for _array_element_2 (.Transforms (Utilities|Struct|BreakSTRUCT_ISM_Save _array_element))
            (CallFunction|AddArrayISM (.StaticMesh (Utilities|Struct|BreakSTRUCT_ISM_Save _array_element)) _array_element_2))))
      (:then_1
        (for _array_element_3 (Variables|/Game/MapEditorExample/Blueprints/Saving/Editor_SaveGame.Editor_SaveGame_C|GetActors (LocalVariables|GetEditorSaveGame))
          (bind _returnvalue_3 (Game|SpawnActorfromClass (.Class (Utilities|Struct|BreakSTRUCT_Actor_Save _array_element_3)) (.Transform (Utilities|Struct|BreakSTRUCT_Actor_Save _array_element_3)) true 0))
          (Class|ISaveableActor|LoadActor(Message) _returnvalue_3 _array_element_3))))))