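; Base pawn for the map editor example, providing a camera on a spring arm with switchable RTS and free movement modes.
; Each mode is a Comp_Movement_Base component; ActivateComponent deactivates the current one and activates the new one, starting with RTS and toggled by Space.
; Movement, mouse, zoom and right-click input is forwarded to the active component.
; View getters return the camera's location and the spring arm's rotation.
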(event `ActivateComponent`
  (params (Component :type "ActorComponent Object Reference"))
  (bind _activecomponent (`self.ActiveComponent`))
  (bind _activecomponent_2 (`self.ActiveComponent`))
  (bind _ascomp_movement_base (cast `/Game/MapEditorExample/Blueprints/Pawns/Comp_Movement_Base` Component))
  (`|ExecutionSequence`
    (:`then_0`
      (if (and (`KismetSystemLibrary.IsValid` _activecomponent) (!= _activecomponent _ascomp_movement_base))
        (`ActorComponent.Deactivate` _activecomponent_2)
        (`/Game/MapEditorExample/Blueprints/Pawns/Comp_Movement_Base.DeActivateComp` _activecomponent_2)))
    (:`then_1`
      (bind _output_get (set `self.ActiveComponent` _ascomp_movement_base))
      (`ActorComponent.Activate` _output_get false)
      (`/Game/MapEditorExample/Blueprints/Pawns/Comp_Movement_Base.ActivateComp` _output_get))))

(event `Key|SpaceBar` :consume false :overrideparent false
  (:`Pressed`
    (if (`/Game/MapEditorExample/Blueprints/Pawns/Comp_Movement_Base.bActive` (`self.Comp_Movement_RTS`))
      (`self.ActivateComponent` (`self.Comp_Movement_Free`))
      (else
        (`self.ActivateComponent` (`self.Comp_Movement_RTS`))))))

(event `Key|RightMouseButton` :consume false :overrideparent false
  ;[1 1 1] Movement Component Events
  (:`Pressed`
    (`/Engine/EditorBlueprintResources/StandardMacros.IsValid` (`self.ActiveComponent`)
      (:`Is Valid`
        (`/Game/MapEditorExample/Blueprints/Pawns/Comp_Movement_Base.SecondaryFire` (`self.ActiveComponent`) true))))
  (:`Released`
    (`/Engine/EditorBlueprintResources/StandardMacros.IsValid` (`self.ActiveComponent`)
      (:`Is Valid`
        (`/Game/MapEditorExample/Blueprints/Pawns/Comp_Movement_Base.SecondaryFire` (`self.ActiveComponent`) false)))))

(event `InputAction|CameraZoomIn` :consume false :overrideparent false
  ;[1 1 1] Movement Component Events
  (:`Pressed`
    (`/Engine/EditorBlueprintResources/StandardMacros.IsValid` (`self.ActiveComponent`)
      (:`Is Valid`
        (`/Game/MapEditorExample/Blueprints/Pawns/Comp_Movement_Base.ZoomIn` (`self.ActiveComponent`) true))))
  (:`Released`
    (`/Engine/EditorBlueprintResources/StandardMacros.IsValid` (`self.ActiveComponent`)
      (:`Is Valid`
        (`/Game/MapEditorExample/Blueprints/Pawns/Comp_Movement_Base.ZoomIn` (`self.ActiveComponent`) false)))))

(event `InputAction|CameraZoomOut` :consume false :overrideparent false
  ;[1 1 1] Movement Component Events
  (:`Pressed`
    (`/Engine/EditorBlueprintResources/StandardMacros.IsValid` (`self.ActiveComponent`)
      (:`Is Valid`
        (`/Game/MapEditorExample/Blueprints/Pawns/Comp_Movement_Base.ZoomOut` (`self.ActiveComponent`) true))))
  (:`Released`
    (`/Engine/EditorBlueprintResources/StandardMacros.IsValid` (`self.ActiveComponent`)
      (:`Is Valid`
        (`/Game/MapEditorExample/Blueprints/Pawns/Comp_Movement_Base.ZoomOut` (`self.ActiveComponent`) false)))))

(event `InputAxis|MoveForward` :consume false :overrideparent false
  (params (AxisValue :type "Float (single-precision)"))
  ;[1 1 1] Movement Component Events
  (`/Engine/EditorBlueprintResources/StandardMacros.IsValid` (`self.ActiveComponent`)
    (:`Is Valid`
      (`/Game/MapEditorExample/Blueprints/Pawns/Comp_Movement_Base.MoveForward` (`self.ActiveComponent`) AxisValue))))

(event `InputAxis|MoveRight` :consume false :overrideparent false
  (params (AxisValue :type "Float (single-precision)"))
  ;[1 1 1] Movement Component Events
  (`/Engine/EditorBlueprintResources/StandardMacros.IsValid` (`self.ActiveComponent`)
    (:`Is Valid`
      (`/Game/MapEditorExample/Blueprints/Pawns/Comp_Movement_Base.MoveRight` (`self.ActiveComponent`) AxisValue))))

(event `self.ReceiveBeginPlay`
  (`self.ActivateComponent` (`self.Comp_Movement_RTS`)))

(event `InputAxisKey|MouseX` :consume false :overrideparent false
  (params (AxisValue :type "Float (single-precision)"))
  ;[1 1 1] Movement Component Events
  (`/Engine/EditorBlueprintResources/StandardMacros.IsValid` (`self.ActiveComponent`)
    (:`Is Valid`
      (`/Game/MapEditorExample/Blueprints/Pawns/Comp_Movement_Base.MouseX` (`self.ActiveComponent`) AxisValue))))

(event `InputAxisKey|MouseY` :consume false :overrideparent false
  (params (AxisValue :type "Float (single-precision)"))
  ;[1 1 1] Movement Component Events
  (`/Engine/EditorBlueprintResources/StandardMacros.IsValid` (`self.ActiveComponent`)
    (:`Is Valid`
      (`/Game/MapEditorExample/Blueprints/Pawns/Comp_Movement_Base.MouseY` (`self.ActiveComponent`) AxisValue))))

(event `self.ReceiveActorBeginOverlap`
  (params (OtherActor :type "Actor Object Reference")))

(event `self.ReceiveTick`
  (params (DeltaSeconds :type "Float (single-precision)")))

(fn `GetViewLocation`
  (returns (Location :type "Object.Vector Structure"))
  (return (`SceneComponent.K2_GetComponentLocation` (`self.Camera`))))

(fn `GetViewRotation`
  (returns (Rotation :type "Object.Rotator Structure"))
  (return (`SceneComponent.K2_GetComponentRotation` (`self.SpringArm`))))

(fn `UserConstructionScript`)