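; BP_MasterBuilding is a map editor building that can be previewed, recolored and saved.
; A dynamic material instance drives five meshes, while preview mode swaps in a preview material and disables collision.
; Clicking its selection box sends color options to the player controller, and it offers delete and color modifiers.
; Saves pack class, transform and a delimited string, from which loading parses and reapplies only the color, ignoring the preview flag.
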(event OnClicked(SelectionBox)
  (params (TouchedComponent :type Primitive%20Component%20Object%20Reference))
  (Class|BPIHUDController|PopulateColorButtons(Message) (Game|GetPlayerController 0) (Variables|Default|GetSTRUCT_Colors) self))

(event Custom|PreviewMode
  (params (bIsInPreviewMode :type Boolean :default false))
  (Collision|SetActorEnableCollision (not bIsInPreviewMode))
  (CallFunction|SetMaterial bIsInPreviewMode))

(event EventLoadActor
  (params (Stats :type STRUCT%20Actor%20Save%20Structure))
  (for _array_element (Utilities|String|ParseIntoArray (.SaveString (Utilities|Struct|BreakSTRUCT_Actor_Save Stats)) "$$")
    (if (>= (Utilities|String|FindSubstring _array_element "Color:" true) 0)
      (CallFunction|ParseColor _array_element)
      (elif (>= (Utilities|String|FindSubstring _array_element "Preview:" true) 0)
        _))))

(event EventBeginPlay
  (CallFunction|PreviewMode false))

(event EventApplyColor
  (params (ColorToApply :type Linear%20Color%20Structure))
  (Rendering|Material|SetVectorParameterValue (Variables|Default|GetBuildingMat) "Color" ColorToApply :!class /Script/Engine.MaterialInstanceDynamic)
  (CallFunction|SetMaterial false))

(fn ConstructionScript
  (bind _returnvalue (Rendering|Material|CreateDynamicMaterialInstance "/Game/MapEditorExample/Materials/M_BuildingMaster.M_BuildingMaster" :!class /Script/Engine.KismetMaterialLibrary))
  (Variables|Default|SetBuildingMat _returnvalue)
  (CallFunction|SetMaterial false))

(fn SetMaterial
  (params (bPreviewMode :type Boolean :default false))
  (Rendering|Material|SetMaterial (Variables|Default|GetStaticMesh1) 0 (select bPreviewMode "/Game/MapEditorExample/Materials/M_Preview.M_Preview" (Variables|Default|GetBuildingMat)))
  (return))

(fn ParseColor
  (params (ColorString :type String))
  (bind _returnvalue (Utilities|String|Len "Color:("))
  (for (_array_element _array_index) (Utilities|String|ParseIntoArray (Class|KismetStringLibrary|Mid ColorString _returnvalue (- (- (Utilities|String|Len ColorString) _returnvalue) 1)) ",")
    (switch int _array_index
      (:0
        (Utilities|Struct|SetmembersinLinearColor (LocalVariables|GetColor) (Math|Conversions|ToFloat(Integer) (Class|KismetStringLibrary|Mid _array_element 2 (- (Utilities|String|Len _array_element) 2)))))
      (:1
        (Utilities|Struct|SetmembersinLinearColor (LocalVariables|GetColor) (Math|Conversions|ToFloat(Integer) (Class|KismetStringLibrary|Mid _array_element 2 (- (Utilities|String|Len _array_element) 2)))))
      (:2
        (Utilities|Struct|SetmembersinLinearColor (LocalVariables|GetColor) (Math|Conversions|ToFloat(Integer) (Class|KismetStringLibrary|Mid _array_element 2 (- (Utilities|String|Len _array_element) 2)))))
      (:3
        (Utilities|Struct|SetmembersinLinearColor (LocalVariables|GetColor) (Math|Conversions|ToFloat(Integer) (Class|KismetStringLibrary|Mid _array_element 2 (- (Utilities|String|Len _array_element) 2)))))))
  (CallFunction|ApplyColor (LocalVariables|GetColor)))

(fn GetModifiers
  (return (Utilities|Array|MakeArray "/Game/MapEditorExample/Blueprints/Modifiers/BP_ModifyActor_Delete.BP_ModifyActor_Delete_C" "/Game/MapEditorExample/Blueprints/Modifiers/BP_ModifyActor_Color.BP_ModifyActor_Color_C")))

(fn GetSaveStats
  (bind _returnvalue (Rendering|Material|GetVectorParameterValue (Variables|Default|GetBuildingMat) "Color" :!class /Script/Engine.MaterialInstanceDynamic))
  (return (Utilities|Struct|MakeSTRUCT_Actor_Save (.AsActor (Utilities|Casting|CastToActorClass (Utilities|GetClass self))) (Math|Transform|MakeTransform (Transformation|GetActorLocation) (Transformation|GetActorRotation) (Transformation|GetActorScale3D)) (Utilities|String|Append (Utilities|String|Append (Utilities|String|Append "Color:" (Utilities|String|ToString(Integer) _returnvalue)) "$$") "Preview:False"))))

(fn GetStaticMesh
  (return "/Engine/EngineMeshes/SM_MatPreviewMesh_01.SM_MatPreviewMesh_01"))