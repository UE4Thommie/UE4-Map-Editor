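; BP_Red_Building is a placeable building variant in the map editor example, colored red.
; Its construction script assigns 400x400 modular meshes for walls, one door wall and a floor, then runs the parent construction script.
; Its PreviewMode event calls the parent implementation and applies the red color only when the building is not in preview mode.
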(event `self.PreviewMode`
  (params (bIsInPreviewMode :type Boolean))
  (`parent.PreviewMode` bIsInPreviewMode)
  (if (not bIsInPreviewMode)
    (`self.ApplyColor` (struct :`R` 255.0 :`A` 1.0))))

(fn `UserConstructionScript`
  (`|ExecutionSequence`
    (:`then_0`
      (`StaticMeshComponent.SetStaticMesh` "/Game/StarterContent/Architecture/Wall_400x400.Wall_400x400"))
    (:`then_1`
      (`StaticMeshComponent.SetStaticMesh` "/Game/StarterContent/Architecture/Wall_Door_400x400.Wall_Door_400x400"))
    (:`then_2`
      (`StaticMeshComponent.SetStaticMesh` "/Game/StarterContent/Architecture/Wall_400x400.Wall_400x400"))
    (:`then_3`
      (`StaticMeshComponent.SetStaticMesh` "/Game/StarterContent/Architecture/Wall_400x400.Wall_400x400"))
    (:`then_4`
      (`StaticMeshComponent.SetStaticMesh` "/Game/StarterContent/Architecture/Wall_400x400.Wall_400x400"))
    (:`then_5`
      (`StaticMeshComponent.SetStaticMesh` "/Game/StarterContent/Architecture/Floor_400x400.Floor_400x400"))
    (:`then_6`
      (`parent.UserConstructionScript`))))