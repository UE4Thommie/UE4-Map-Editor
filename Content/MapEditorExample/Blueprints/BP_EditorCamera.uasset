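; Map editor camera that works in either an RTS Style or Free Cam mode.
; On BeginPlay it registers with the player controller, and in Free Cam spawns a DefaultPawn for the controller to possess.
; In RTS Style, Tick interpolates boom length toward a clamped zoom target from mouse wheel or zoom events, and pans the root by yaw-rotated axis values.
; Per-mode camera and boom setup sits disconnected in the construction script.
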(event `self.ReceiveBeginPlay`
  (message `/Game/MapEditorExample/Blueprints/Interfaces/BPI_Camera_Controller.SetCamera` (`GameplayStatics.GetPlayerController` 0) self)
  (switch `/Game/MapEditorExample/Blueprints/Enums/ECameraMode` (`self.CameraMode`)
    (:`NewEnumerator0`
      (bind _returnvalue (`|SpawnActorFromClass` "/Script/Engine.DefaultPawn" (`self.GetTransform`)))
      (message `/Game/MapEditorExample/Blueprints/Interfaces/BPI_Camera_Controller.PossessDefaultPawn` (`GameplayStatics.GetPlayerController` 0) _returnvalue))))

(event `self.ReceiveTick`
  (params (DeltaSeconds :type "Float (single-precision)"))
  (bind _mainroot (`self.MainRoot`))
  (bind _cameraboom (`self.CameraBoom`))
  ;[1 1 1] Zoom Interp
  (switch `/Game/MapEditorExample/Blueprints/Enums/ECameraMode` (`self.CameraMode`)
    (:`NewEnumerator1`
      (set `SpringArmComponent.TargetArmLength` (`KismetMathLibrary.FInterpTo` (`SpringArmComponent.TargetArmLength` _cameraboom) (`self.BoomLength`) 0.1 (`self.ZoomSpeed`)) _cameraboom)
      ;[1 1 1] Camera WASD Movement
      (bind _output_get (set `self.CameraPan` (`KismetMathLibrary.MakeVector` (`self.ForwardAxis`) (`self.RightAxis`))))
      (bind _output_get_2 (set `self.CameraPan` (* (`KismetMathLibrary.GreaterGreater_VectorRotator` _output_get (`KismetMathLibrary.MakeRot` 0.0 (.yaw (`SceneComponent.K2_GetComponentRotation` _mainroot)))) (`self.WASDSpeed`))))
      (`SceneComponent.K2_SetWorldLocation` (`self.MainRoot`) (+ (`SceneComponent.K2_GetComponentLocation` _mainroot) _output_get_2) false))))

(event `Key|MouseScrollUp` :consume false
  (:`Pressed`
    (set `self.BoomLength` (`KismetMathLibrary.FClamp` (- (`SpringArmComponent.TargetArmLength` (`self.CameraBoom`)) 300.0) 0.0 4000.0) :!label _label)))

(event `ZoomIn`
  (goto _label))

(event `ZoomOut`
  (set `self.BoomLength` (`KismetMathLibrary.FClamp` (+ (`SpringArmComponent.TargetArmLength` (`self.CameraBoom`)) 300.0) 0.0 4000.0) :!label _label_2))

(event `Key|MouseScrollDown` :consume false
  (:`Pressed`
    (goto _label_2)))

(fn `GetCameraMode`
  (returns (Mode :type "/Game/MapEditorExample/Blueprints/Enums/ECameraMode Enum"))
  (return (`self.CameraMode`)))

(fn `UserConstructionScript`)