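; RTS-style camera movement component for the map editor pawn, handling pan, zoom and yaw rotation.
; On activation it tilts the spring arm and traces along its view to set the starting target location and distance.
; Input shifts those targets with curve-based, distance-scaled speeds, while secondary fire enables mouse rotation.
; Tick interpolates position and arm length, snapping the pawn to Camera-channel surfaces with a vertical trace.
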(event `self.SecondaryFire`
  (params (bPressed :type Boolean))
  (set `self.bShouldRotate` bPressed))

(event `self.ActivateComp`
  (bind _returnvalue (`self.GetOwner`))
  (bind (_returnvalue_pitch _returnvalue_yaw) (`KismetMathLibrary.BreakRotator` (`Actor.K2_GetActorRotation` _returnvalue)))
  (bind _returnvalue_2 (`Actor.K2_GetActorLocation` (`self.GetOwner`)))
  (bind _returnvalue_3 (+ _returnvalue_2 (* (`KismetMathLibrary.GetForwardVector` (`SceneComponent.K2_GetComponentRotation` (`self.SpringArm`))) (`self.MaxDistance`))))
  (`|ExecutionSequence`
    (:`then_0`
      (`/Engine/EditorBlueprintResources/StandardMacros.IsValid` (`self.GetOwner`)
        (:`Is Valid`
          (bind _aspawn_editor_base (cast `/Game/MapEditorExample/Blueprints/Pawns/Pawn_Editor_Base` (`self.GetOwner`)))
          (bind _output_get (set `self.SpringArm` (`/Game/MapEditorExample/Blueprints/Pawns/Pawn_Editor_Base.SpringArm` _aspawn_editor_base)))
          (bind (_relativerotation_pitch _relativerotation_yaw _relativerotation_roll) (`KismetMathLibrary.BreakRotator` (`SceneComponent.RelativeRotation` _output_get)))
          (`SceneComponent.K2_SetRelativeRotation` _output_get (`KismetMathLibrary.MakeRotator` -50.0 _relativerotation_yaw _relativerotation_roll) false)
          (`Actor.SetActorRotation` _returnvalue (`KismetMathLibrary.MakeRotator` 0.0 _returnvalue_yaw))
          (bind (_outhit _returnvalue_4) (`KismetSystemLibrary.LineTraceSingle` _returnvalue_2 _returnvalue_3 "TraceTypeQuery1" true))
          (if _returnvalue_4
            (bind (_bblockinghit _time _location) (`GameplayStatics.BreakHitResult` _outhit))
            (set `self.TargetDistance` (`KismetMathLibrary.VSize` (- (`Actor.K2_GetActorLocation` (`self.GetOwner`)) _location)))
            (set `self.TargetLocation` _location)
            (else
              (set `self.TargetDistance` (`self.MaxDistance`))
              (set `self.TargetLocation` _returnvalue_3))))))
    (:`then_1`
      (`parent.ActivateComp`))))

(event `self.ZoomIn`
  (params (bPressed :type Boolean))
  ;[1 1 1] Zoom events
  (if bPressed
    (set `self.TargetDistance` (`KismetMathLibrary.FClamp` (- (`self.TargetDistance`) (* (`CurveFloat.GetFloatValue` (`self.ZoomCurve`) (`self.TargetDistance`)) (`self.ZoomSpeed`))) (`self.MinDistance`) (`self.MaxDistance`)))))

(event `self.ZoomOut`
  (params (bPressed :type Boolean))
  ;[1 1 1] Zoom events
  (if bPressed
    (set `self.TargetDistance` (`KismetMathLibrary.FClamp` (+ (`self.TargetDistance`) (* (`CurveFloat.GetFloatValue` (`self.ZoomCurve`) (`self.TargetDistance`)) (`self.ZoomSpeed`))) (`self.MinDistance`) (`self.MaxDistance`)))))

(event `self.MoveForward`
  (params (Value :type "Float (single-precision)"))
  ;[1 1 1] Default Movement / Set actor location
  (set `self.TargetLocation` (+ (`self.TargetLocation`) (* (* (`KismetMathLibrary.Normal` (`KismetMathLibrary.Conv_DoubleToVector` Value)) (`KismetMathLibrary.GetForwardVector` (`Actor.K2_GetActorRotation` (`self.GetOwner`)))) (* (`CurveFloat.GetFloatValue` (`self.MoveCurve`) (`self.TargetDistance`)) (`self.MoveSpeed`))) (* (* (`KismetMathLibrary.Normal` (`KismetMathLibrary.Conv_DoubleToVector` (stale `self.MoveRight` Value))) (`KismetMathLibrary.GetRightVector` (`Actor.K2_GetActorRotation` (`self.GetOwner`)))) (* (`CurveFloat.GetFloatValue` (`self.MoveCurve`) (`self.TargetDistance`)) (`self.MoveSpeed`)))) :!label _label))

(event `self.ReceiveInitializeComponent`)

(event `self.MoveRight`
  (params (Value :type "Float (single-precision)"))
  (goto _label))

(event `self.MouseX`
  (params (Value :type "Float (single-precision)"))
  ;[1 1 1] Rotation
  (if (`self.bShouldRotate`)
    (`Actor.K2_AddActorWorldRotation` (`self.GetOwner`) (`KismetMathLibrary.MakeRot` 0.0 (* Value (`self.RotationSpeed`))) false)))

(event `self.ReceiveTick`
  (params (DeltaSeconds :type "Float (single-precision)"))
  (bind _returnvalue (`Actor.K2_GetActorLocation` (`self.GetOwner`)))
  (if (`self.bActive`)
    (`|ExecutionSequence`
      (:`then_0`
        (`Actor.K2_SetActorLocation` (`self.GetOwner`) (`KismetMathLibrary.VInterpTo` (`Actor.K2_GetActorLocation` (`self.GetOwner`)) (`self.TargetLocation`) DeltaSeconds 100.0) false))
      (:`then_1`
        ;[1 1 1] Set Camera location
        (bind _outhit (`KismetSystemLibrary.LineTraceSingle` (+ _returnvalue (0.0 0.0 500000.0)) (- _returnvalue (0.0 0.0 500000.0)) "TraceTypeQuery2" true))
        (`Actor.K2_SetActorLocation` (`self.GetOwner`) (`.Location` (`GameplayStatics.BreakHitResult` _outhit)) false))
      (:`then_2`
        ;[1 1 1] Zooming
        (set `SpringArmComponent.TargetArmLength` (`KismetMathLibrary.FInterpTo` (`SpringArmComponent.TargetArmLength` (`self.SpringArm`)) (`self.TargetDistance`) DeltaSeconds 10.0) (`self.SpringArm`))))))