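; Map editor modifier actor that recolors a building when activated.
; On Activate it runs the parent logic, then casts its valid RelatedActor to BP_MasterBuilding and calls ApplyColor with a random opaque color.
; Random RGB channels are drawn from a 0–255 range into a linear color rather than 0–1.
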(event `self.ReceiveBeginPlay`
  (`parent.ReceiveBeginPlay`))

(event `self.ReceiveActorBeginOverlap`
  (params (OtherActor :type "Actor Object Reference")))

(event `self.ReceiveTick`
  (params (DeltaSeconds :type "Float (single-precision)"))
  (`parent.ReceiveTick` 0.0))

(event `self.Activate`
  (params (Actor :type "Actor Object Reference"))
  (`parent.Activate` Actor)
  (`/Engine/EditorBlueprintResources/StandardMacros.IsValid` (`self.RelatedActor`)
    (:`Is Valid`
      (bind _asbp_master_building (cast `/Game/MapEditorExample/Blueprints/Buildings/BP_MasterBuilding` (`self.RelatedActor`)))
      (`/Game/MapEditorExample/Blueprints/Buildings/BP_MasterBuilding.ApplyColor` _asbp_master_building (make `Object.LinearColor` (`KismetMathLibrary.RandomFloatInRange` 0.0 255.0) (`KismetMathLibrary.RandomFloatInRange` 0.0 255.0) (`KismetMathLibrary.RandomFloatInRange` 0.0 255.0) 1.0)))))

(fn `UserConstructionScript`
  (`parent.UserConstructionScript`))