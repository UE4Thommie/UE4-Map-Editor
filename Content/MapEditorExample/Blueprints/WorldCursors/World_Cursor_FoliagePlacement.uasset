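; Map editor world cursor that paints a chosen foliage mesh while the left mouse button is held.
; It follows the mouse hit location and repeats PaintFoliage on a looping timer until release.
; Each stroke adds a random number of randomly yawed and scaled meshes through the SaveGameManager.
; Placement projects random points from the cursor mesh bounds onto the impact-point vector of an upward sphere trace.
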(event `Key|LeftMouseButton`
  (:`Pressed`
    (`self.PaintFoliage`) ; First stroke
    (`KismetSystemLibrary.K2_SetTimer` self "PaintFoliage" 0.2 true))
  (:`Released`
    (`KismetSystemLibrary.K2_ClearTimer` self "PaintFoliage")))

(event `Initialize`
  (params (`Static Mesh` :type "StaticMesh Object Reference") (SGManager :type "/Game/MapEditorExample/Blueprints/Saving/SaveGame_Manager Object Reference"))
  (`/Engine/EditorBlueprintResources/StandardMacros.IsValid` `Static Mesh`
    (:`Is Valid`
      (set `self.FoliageMesh` `Static Mesh`)
      (set `self.SaveGameManager` SGManager))
    (:`Is Not Valid`
      (`self.K2_DestroyActor`))))

(event `self.GetMouseHitInfo`
  (params (Location :type "Object.Vector Structure") (Actor :type "Actor Object Reference") (Component :type "PrimitiveComponent Object Reference"))
  (`/Engine/EditorBlueprintResources/StandardMacros.IsValid` (`self.FoliageMesh`)
    (:`Is Valid`
      (`self.K2_SetActorLocation` Location))))

(event `PaintFoliage`
  (bind _returnvalue (`self.K2_GetActorLocation`))
  (bind _minscale (`self.MinScale`))
  (bind _maxscale (`self.MaxScale`))
  (bind (_origin _boxextent _sphereradius) (`KismetSystemLibrary.GetComponentBounds` (`self.StaticMesh`)))
  (for _ (range 1 (+ (`KismetMathLibrary.RandomIntegerInRange` 1 (`self.MaxFoliageCount`)) 1))
    (bind _outhit (`KismetSystemLibrary.SphereTraceSingle_NEW` _returnvalue (+ _returnvalue (* (`self.GetActorUpVector`) 100.0)) (/ _sphereradius 2.0) "TraceTypeQuery1"))
    (`/Game/MapEditorExample/Blueprints/Saving/SaveGame_Manager.AddStaticMesh` (`self.SaveGameManager`) (`self.FoliageMesh`) (`KismetMathLibrary.MakeTransform` (`KismetMathLibrary.ProjectVectorOnToVector` (`KismetMathLibrary.RandomPointInBoundingBox` _origin _boxextent) (`.ImpactPoint` (`GameplayStatics.BreakHitResult` _outhit))) (`KismetMathLibrary.MakeRot` 0.0 (`KismetMathLibrary.RandomFloatInRange` 0.0 360.0)) (`KismetMathLibrary.MakeVector` (`KismetMathLibrary.RandomFloatInRange` _minscale _maxscale) (`KismetMathLibrary.RandomFloatInRange` _minscale _maxscale) (`KismetMathLibrary.RandomFloatInRange` _minscale _maxscale))))))

(event `self.ReceiveBeginPlay`)

(event `self.ReceiveActorBeginOverlap`
  (params (OtherActor :type "Actor Object Reference")))

(event `self.ReceiveTick`
  (params (DeltaSeconds :type "Float (single-precision)")))

(fn `UserConstructionScript`
  (`parent.UserConstructionScript`))