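; Free-fly movement component for the map editor pawn, with zoom inputs repurposed to adjust movement speed.
; On activation it targets the camera's position and transfers the spring arm's rotation to the actor.
; Movement inputs shift a target location along the arm's axes, which Tick interpolates toward while easing arm length to TargetDistance.
; Holding secondary fire enables mouse look, using world-space yaw and local pitch to avoid roll.
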(event `self.ZoomIn`
  (params (bPressed :type Boolean))
  (if bPressed
    (set `self.MovementSpeed` (`KismetMathLibrary.FClamp` (+ (`self.MovementSpeed`) 20.0) (`self.MinSpeed`) (`self.MaxSpeed`)))))

(event `self.ZoomOut`
  (params (bPressed :type Boolean))
  (if bPressed
    (set `self.MovementSpeed` (`KismetMathLibrary.FClamp` (- (`self.MovementSpeed`) 20.0) (`self.MinSpeed`) (`self.MaxSpeed`)))))

(event `self.ActivateComp`
  (`|ExecutionSequence`
    (:`then_0`
      (`/Engine/EditorBlueprintResources/StandardMacros.IsValid` (`self.GetOwner`)
        (:`Is Valid`
          (bind _aspawn_editor_base (cast `/Game/MapEditorExample/Blueprints/Pawns/Pawn_Editor_Base` (`self.GetOwner`)))
          (set `self.Sphere` (`/Game/MapEditorExample/Blueprints/Pawns/Pawn_Editor_Base.Sphere` _aspawn_editor_base))
          (bind _output_get (set `self.SpringArm` (`/Game/MapEditorExample/Blueprints/Pawns/Pawn_Editor_Base.SpringArm` _aspawn_editor_base)))
          (`|ExecutionSequence`
            (:`then_0`
              (set `self.TargetLocation` (- (`Actor.K2_GetActorLocation` (`self.GetOwner`)) (* (`KismetMathLibrary.GetForwardVector` (`SceneComponent.K2_GetComponentRotation` _output_get)) (`SpringArmComponent.TargetArmLength` _output_get)))))
            (:`then_1`
              (bind (_returnvalue_pitch _returnvalue_yaw) (`KismetMathLibrary.BreakRotator` (`SceneComponent.K2_GetComponentRotation` _output_get)))
              (`Actor.SetActorRotation` (`self.GetOwner`) (`KismetMathLibrary.MakeRotator` _returnvalue_pitch _returnvalue_yaw))
              (`SceneComponent.K2_SetRelativeRotation` :`self` _output_get))))))
    (:`then_1`
      (`parent.ActivateComp`))))

(event `self.ReceiveTick`
  (params (DeltaSeconds :type "Float (single-precision)"))
  (if (`self.bActive`)
    (`Actor.K2_SetActorLocation` (`self.GetOwner`) (`KismetMathLibrary.VInterpTo` (`Actor.K2_GetActorLocation` (`self.GetOwner`)) (`self.TargetLocation`) DeltaSeconds 100.0) false)
    ;[1 1 1] Zooming
    (set `SpringArmComponent.TargetArmLength` (`KismetMathLibrary.FInterpTo` (`SpringArmComponent.TargetArmLength` (`self.SpringArm`)) (`self.TargetDistance`) DeltaSeconds 10.0) (`self.SpringArm`))))

(event `self.ReceiveInitializeComponent`)

(event `self.MoveForward`
  (params (Value :type "Float (single-precision)"))
  (bind _springarm (`self.SpringArm`))
  (set `self.TargetLocation` (+ (`self.TargetLocation`) (* (* (`KismetMathLibrary.Normal` (`KismetMathLibrary.Conv_DoubleToVector` Value)) (`KismetMathLibrary.GetForwardVector` (`SceneComponent.K2_GetComponentRotation` _springarm))) (`self.MovementSpeed`)) (* (* (`KismetMathLibrary.Normal` (`KismetMathLibrary.Conv_DoubleToVector` (stale `self.MoveRight` Value))) (`KismetMathLibrary.GetRightVector` (`SceneComponent.K2_GetComponentRotation` _springarm))) (`self.MovementSpeed`))) :!label _label))

(event `self.MoveRight`
  (params (Value :type "Float (single-precision)"))
  (goto _label))

(event `self.SecondaryFire`
  (params (bPressed :type Boolean))
  (set `self.bShouldRotate` bPressed))

(event `self.MouseX`
  (params (Value :type "Float (single-precision)"))
  (if (`self.bShouldRotate`)
    (`Actor.K2_AddActorWorldRotation` (`self.GetOwner`) (`KismetMathLibrary.MakeRotator` 0.0 (* Value (`self.RotationSpeed`))) false)))

(event `self.MouseY`
  (params (Value :type "Float (single-precision)"))
  (if (`self.bShouldRotate`)
    (`Actor.K2_AddActorLocalRotation` (`self.GetOwner`) (`KismetMathLibrary.MakeRotator` (* Value (`self.RotationSpeed`))) false)))