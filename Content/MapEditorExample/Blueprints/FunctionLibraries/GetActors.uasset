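; Blueprint function library in the map editor example that gives global access to two singleton-style actors: the save game manager and the settings actor.
; GetSaveGameManager and GetSettings each run GetAllActorsOfClass for SaveGame_Manager or BP_Settings and return the first instance found.
; Each call searches the world again, and the result is left unset if no such actor exists.
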(fn GetSaveGameManager
  (Utilities|FlowControl|Sequence
    (:then_0
      (bind _outactors (Actor|GetAllActorsOfClass 0 "/Game/MapEditorExample/Blueprints/Saving/SaveGame_Manager.SaveGame_Manager_C"))
      (if (> (Utilities|Array|Length _outactors) 0)
        (LocalVariables|SetManager (Utilities|Array|Get(acopy) _outactors))))
    (:then_1
      (return (LocalVariables|GetManager)))))

(fn GetSettings
  (Utilities|FlowControl|Sequence
    (:then_0
      (bind _outactors (Actor|GetAllActorsOfClass 0 "/Game/MapEditorExample/Blueprints/Settings/BP_Settings.BP_Settings_C"))
      (if (> (Utilities|Array|Length _outactors) 0)
        (LocalVariables|SetaSettings (Utilities|Array|Get(acopy) _outactors))))
    (:then_1
      (return (LocalVariables|GetaSettings)))))