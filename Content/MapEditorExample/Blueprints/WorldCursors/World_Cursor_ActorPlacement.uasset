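; World cursor for the map editor example that previews and places an actor of a given class.
; Initialize spawns a temporary instance to borrow its mesh through I_SaveableActor, applies M_Preview, then destroys the instance; classes without the interface are rejected.
; GetMouseHitInfo moves the preview to the hit location with sweep.
; Left click spawns the target class at the cursor's location and rotation, then destroys the cursor.
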(event `Key|LeftMouseButton`
  (:`Pressed`
    (if (`KismetSystemLibrary.IsValidClass` (`self.TargetClass`))
      (`|SpawnActorFromClass` (`self.TargetClass`) (`KismetMathLibrary.MakeTransform` (`self.K2_GetActorLocation`) (`self.K2_GetActorRotation`)) true)
      (`self.K2_DestroyActor`))))

(event `self.GetMouseHitInfo`
  (params (Location :type "Object.Vector Structure") (Actor :type "Actor Object Reference") (Component :type "PrimitiveComponent Object Reference"))
  (if (!= (`self.StaticMesh`) null)
    (`self.K2_SetActorLocation` Location true)))

(event `Initialize`
  (params (ActorClass :type "Actor Class Reference"))
  (bind _returnvalue (`|SpawnActorFromClass` ActorClass (`KismetMathLibrary.MakeTransform` (0.0 0.0 0.0)) true))
  (if (`KismetSystemLibrary.DoesImplementInterface` _returnvalue "/Game/MapEditorExample/Blueprints/Saving/I_SaveableActor.I_SaveableActor_C")
    (bind _visiblemesh (message `/Game/MapEditorExample/Blueprints/Saving/I_SaveableActor.GetStaticMesh` _returnvalue))
    (`StaticMeshComponent.SetStaticMesh` _visiblemesh)
    (`self.K2_DestroyActor` _returnvalue)
    (set `self.TargetClass` ActorClass)
    (`PrimitiveComponent.SetMaterial` 0 "/Game/MapEditorExample/Materials/M_Preview.M_Preview")
    (else
      (`self.K2_DestroyActor` _returnvalue))))

(event `self.ReceiveBeginPlay`)

(event `self.ReceiveActorBeginOverlap`
  (params (OtherActor :type "Actor Object Reference")))

(event `self.ReceiveTick`
  (params (DeltaSeconds :type "Float (single-precision)")))

(fn `UserConstructionScript`
  (`parent.UserConstructionScript`))