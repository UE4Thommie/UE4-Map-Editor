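; Map editor rotation gizmo that turns RelatedActor around its local X, Y or Z axis with the mouse.
; Clicking a color-coded, hover-highlighted handle sets the axis; mouse movement rotates the gizmo until left-button release, and Tick copies its rotation to the actor.
; Ctrl+Z and Ctrl+Y step through undo and repeat rotation arrays when not dragging.
; UpdateSensitivity is empty; its distance-based sensitivity and scaling logic is disconnected.
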(event `Key|Ctrl+Z`
  (bind _undoarray (`self.UndoArray`))
  (bind _returnvalue (`KismetArrayLibrary.Array_LastIndex` _undoarray))
  (bind _item (`KismetArrayLibrary.Array_Get` _undoarray _returnvalue))
  ;[1 1 1] Undo/Repeat
  (:`Pressed`
    (if (< (`self.MoveDirection`) 0)
      (if (> (`KismetArrayLibrary.Array_Length` (`self.UndoArray`)) 0)
        (`self.SetActorRotation` _item)
        (`KismetArrayLibrary.Array_Add` (`self.RepeatArray`) _item)
        (`KismetArrayLibrary.Array_Remove` (`self.UndoArray`) _returnvalue)))))

(event `self.DeActivate`
  (bind _relatedactor (`self.RelatedActor`))
  (`|ExecutionSequence`
    (:`then_0`
      (`/Engine/EditorBlueprintResources/StandardMacros.IsValid` (`self.RelatedActor`)
        (:`Is Valid`
          (`self.SetActorEnableCollision` _relatedactor true)
          (`self.SetActorHiddenInGame` _relatedactor false))))
    (:`then_1`
      (`parent.DeActivate`))))

(event `Key|Ctrl+Y`
  (bind _repeatarray (`self.RepeatArray`))
  (bind _returnvalue (`KismetArrayLibrary.Array_LastIndex` _repeatarray))
  (bind _item (`KismetArrayLibrary.Array_Get` _repeatarray _returnvalue))
  ;[1 1 1] Undo/Repeat
  (:`Pressed`
    (if (< (`self.MoveDirection`) 0)
      (if (> (`KismetArrayLibrary.Array_Length` (`self.RepeatArray`)) 0)
        (`self.SetActorRotation` _item)
        (`KismetArrayLibrary.Array_Add` (`self.UndoArray`) _item)
        (`KismetArrayLibrary.Array_Remove` (`self.RepeatArray`) _returnvalue)))))

(event `self.Activate`
  (`parent.Activate`)
  (`self.SetActorEnableCollision` (`self.RelatedActor`) false)
  (`self.SetActorRotation` (`self.K2_GetActorRotation` (`self.RelatedActor`))))

(event `Key|LeftMouseButton`
  (:`Released`
    (set `self.MoveDirection` -1) ; Disable movement
  ))

(event `self.ReceiveActorBeginOverlap`
  (params (OtherActor :type "Actor Object Reference")))

(event `self.ReceiveTick`
  (params (DeltaSeconds :type "Float (single-precision)"))
  (`self.UpdateSensitivity`)
  (`/Engine/EditorBlueprintResources/StandardMacros.IsValid` (`self.RelatedActor`)
    (:`Is Valid`
      (`self.SetActorRotation` (`self.RelatedActor`) (`self.K2_GetActorRotation`)))))

(event `InputAxisKey|MouseX`
  (params (AxisValue :type "Float (single-precision)"))
  (`self.RotateRelatedActor` AxisValue (stale `InputAxisKey|MouseY` AxisValue) :!label _label))

(event `InputAxisKey|MouseY`
  (params (AxisValue :type "Float (single-precision)"))
  (goto _label))

(event `self.Direction_X.OnClicked`
  (params (TouchedComponent :type "PrimitiveComponent Object Reference"))
  ;[1 1 1] Movement modes
  (set `self.MoveDirection` 0)
  (`self.EnableInput` (`self.OwnerPC`) :!label _label_2)
  (`KismetArrayLibrary.Array_Add` (`self.UndoArray`) (`self.K2_GetActorRotation`)))

(event `self.Direction_Y.OnClicked`
  (params (TouchedComponent :type "PrimitiveComponent Object Reference"))
  ;[1 1 1] Movement modes
  (set `self.MoveDirection` 1)
  (goto _label_2))

(event `self.Direction_Z.OnClicked`
  (params (TouchedComponent :type "PrimitiveComponent Object Reference"))
  ;[1 1 1] Movement modes
  (set `self.MoveDirection` 2)
  (goto _label_2))

(event `self.Direction_Z.OnBeginCursorOver`
  (params (TouchedComponent :type "PrimitiveComponent Object Reference"))
  ;[1 1 1] Cursor Hovering
  (`MaterialInstanceDynamic.SetVectorParameterValue` (`self.MID_Z`) "Color" (struct :`R` 255.0 :`G` 255.0 :`A` 1.0)))

(event `self.Direction_Z.OnEndCursorOver`
  (params (TouchedComponent :type "PrimitiveComponent Object Reference"))
  ;[1 1 1] Cursor Hovering
  (`MaterialInstanceDynamic.SetVectorParameterValue` (`self.MID_Z`) "Color" (struct :`B` 255.0 :`A` 1.0)))

(event `self.Direction_Y.OnBeginCursorOver`
  (params (TouchedComponent :type "PrimitiveComponent Object Reference"))
  ;[1 1 1] Cursor Hovering
  (`MaterialInstanceDynamic.SetVectorParameterValue` (`self.MID_Y`) "Color" (struct :`R` 255.0 :`G` 255.0 :`A` 1.0)))

(event `self.Direction_Y.OnEndCursorOver`
  (params (TouchedComponent :type "PrimitiveComponent Object Reference"))
  ;[1 1 1] Cursor Hovering
  (`MaterialInstanceDynamic.SetVectorParameterValue` (`self.MID_Y`) "Color" (struct :`G` 255.0 :`A` 1.0)))

(event `self.Direction_X.OnBeginCursorOver`
  (params (TouchedComponent :type "PrimitiveComponent Object Reference"))
  ;[1 1 1] Cursor Hovering
  (`MaterialInstanceDynamic.SetVectorParameterValue` (`self.MID_X`) "Color" (struct :`R` 255.0 :`G` 255.0 :`A` 1.0)))

(event `self.Direction_X.OnEndCursorOver`
  (params (TouchedComponent :type "PrimitiveComponent Object Reference"))
  ;[1 1 1] Cursor Hovering
  (`MaterialInstanceDynamic.SetVectorParameterValue` (`self.MID_X`) "Color" (struct :`R` 255.0 :`A` 1.0)))

(fn `RotateRelatedActor`
  (params (X :type "Float (double-precision)" :default 0.0) (Y :type "Float (double-precision)" :default 0.0))
  (bind _returnvalue (* (+ X Y) -1.0))
  (switch `int` (`self.MoveDirection`)
    (:`0`
      (`self.K2_AddActorLocalRotation` (`KismetMathLibrary.MakeRot` 0.0 0.0 _returnvalue)))
    (:`1`
      (`self.K2_AddActorLocalRotation` (`KismetMathLibrary.MakeRot` _returnvalue)))
    (:`2`
      (`self.K2_AddActorLocalRotation` (`KismetMathLibrary.MakeRot` 0.0 _returnvalue)))))

(fn `UpdateSensitivity`)

(fn `UserConstructionScript`
  (`parent.UserConstructionScript`)
  (`|ExecutionSequence`
    (:`then_0`
      (bind _returnvalue (`KismetMaterialLibrary.CreateDynamicMaterialInstance` "/Game/MapEditorExample/Materials/M_Color.M_Color"))
      (bind _output_get (set `self.MID_X` _returnvalue))
      (`PrimitiveComponent.SetMaterial` (`self.Direction_X`) 0 _output_get)
      (`MaterialInstanceDynamic.SetVectorParameterValue` (`self.MID_X`) "Color" (struct :`R` 255.0 :`A` 1.0)))
    (:`then_1`
      (bind _returnvalue_2 (`KismetMaterialLibrary.CreateDynamicMaterialInstance` "/Game/MapEditorExample/Materials/M_Color.M_Color"))
      (bind _output_get_2 (set `self.MID_Y` _returnvalue_2))
      (`PrimitiveComponent.SetMaterial` (`self.Direction_Y`) 0 _output_get_2)
      (`MaterialInstanceDynamic.SetVectorParameterValue` (`self.MID_Y`) "Color" (struct :`G` 255.0 :`A` 1.0)))
    (:`then_2`
      (bind _returnvalue_3 (`KismetMaterialLibrary.CreateDynamicMaterialInstance` "/Game/MapEditorExample/Materials/M_Color.M_Color"))
      (bind _output_get_3 (set `self.MID_Z` _returnvalue_3))
      (`PrimitiveComponent.SetMaterial` (`self.Direction_Z`) 0 _output_get_3)
      (`MaterialInstanceDynamic.SetVectorParameterValue` (`self.MID_Z`) "Color" (struct :`B` 255.0 :`A` 1.0)))))