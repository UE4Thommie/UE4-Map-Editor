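; Base actor for map editor modifiers that act on a selected actor, with an optional button widget and secondary menu.
; It stays hidden and inert until activated, then moves to the related actor, takes over its collision and caches the owner pawn's view each tick.
; Advanced activation registers it as the controller's active modifier and opens the menu.
; Deactivation restores the actor's collision and closes the menu.
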(event `AdvancedActivate`
  (`|ExecutionSequence`
    (:`then_0`
      (if (and (not (`self.bActive`)) (`KismetSystemLibrary.IsValid` (`self.RelatedActor`)) (`KismetSystemLibrary.IsValid` (`self.OwnerPC`)))
        (bind _aseditor_controller (cast `/Game/MapEditorExample/Blueprints/Editor_Controller` (`self.OwnerPC`)))
        (`/Game/MapEditorExample/Blueprints/Editor_Controller.SetActiveModifier` _aseditor_controller self (`self.RelatedActor`))))
    (:`then_1`
      (`/Engine/EditorBlueprintResources/StandardMacros.IsValid` (`self.SecondaryWidget`)
        (:`Is Valid`
          (bind _aseditor_controller_2 (cast `/Game/MapEditorExample/Blueprints/Editor_Controller` (`self.OwnerPC`)))
          (`/Game/MapEditorExample/Blueprints/Editor_Controller.Set Menu` _aseditor_controller_2 (`self.SecondaryWidget`)))))))

(event `DeActivate`
  (bind _secondarywidget (`self.SecondaryWidget`))
  (if (`self.bActive`)
    (set `self.bActive` false)
    (`self.DisableInput` (`self.OwnerPC`))
    (`self.SetActorHiddenInGame` true)
    (`self.SetActorEnableCollision` false)
    (`self.SetActorEnableCollision` (`self.RelatedActor`) true)
    (`self.SetActorTickEnabled` false)
    (`/Engine/EditorBlueprintResources/StandardMacros.IsValid` _secondarywidget
      (:`Is Valid`
        (if (`Widget.IsVisible` _secondarywidget)
          (`/Game/MapEditorExample/Blueprints/Modifiers/BP_Modify_Menu_Base.Closed` _secondarywidget _secondarywidget))))))

(event `Activate`
  (params (Actor :type "Actor Object Reference"))
  (if (not (`self.bActive`))
    (set `self.bActive` true)
    (set `self.RelatedActor` Actor)
    (`/Engine/EditorBlueprintResources/StandardMacros.IsValid` (`self.RelatedActor`)
      (:`Is Valid`
        (`self.SetActorHiddenInGame` false)
        (`self.SetActorEnableCollision` true)
        (`self.SetActorEnableCollision` (`self.RelatedActor`) false)
        (`self.SetActorTickEnabled` true)
        (`self.K2_SetActorLocation` (`self.K2_GetActorLocation` (`self.RelatedActor`)))))))

(event `self.ReceiveBeginPlay`
  (bind _primarywidget (`self.PrimaryWidget`))
  (bind _primarywidgetclass (`self.PrimaryWidgetClass`))
  (bind _secondarywidgetclass (`self.SecondaryWidgetClass`))
  (`self.SetActorTickEnabled` false)
  (`self.SetActorEnableCollision` false)
  (`self.SetActorHiddenInGame` true)
  (`|ExecutionSequence`
    (:`then_0`
      (if (`KismetSystemLibrary.IsValidClass` _primarywidgetclass)
        (bind _returnvalue (`|CreateWidget` _primarywidgetclass (`self.OwnerPC`)))
        (bind _asbp_modify_button_base (cast `/Game/MapEditorExample/Blueprints/Modifiers/BP_Modify_Button_Base` _returnvalue))
        (bind _output_get (set `self.PrimaryWidget` _asbp_modify_button_base))
        (`TextBlock.SetText` (`/Game/MapEditorExample/Blueprints/Modifiers/BP_Modify_Button_Base.Main_Txt` _output_get) (`self.PrimaryWidgetText`))))
    (:`then_1`
      (if (`KismetSystemLibrary.IsValidClass` _secondarywidgetclass)
        (bind _returnvalue_2 (`|CreateWidget` _secondarywidgetclass (`self.OwnerPC`)))
        (bind _asbp_modify_menu_base (cast `/Game/MapEditorExample/Blueprints/Modifiers/BP_Modify_Menu_Base` _returnvalue_2))
        (set `self.SecondaryWidget` _asbp_modify_menu_base)
        (`/Engine/EditorBlueprintResources/StandardMacros.IsValid` _primarywidget
          (:`Is Valid`
            (add `/Game/MapEditorExample/Blueprints/Modifiers/BP_Modify_Button_Base.OnRMBPress` _primarywidget (`|CreateDelegate` self :!event `AdvancedActivate`))))))))

(event `self.ReceiveActorBeginOverlap`
  (params (OtherActor :type "Actor Object Reference")))

(event `self.ReceiveTick`
  (params (DeltaSeconds :type "Float (single-precision)"))
  (bind _returnvalue (`Controller.K2_GetPawn` (`self.OwnerPC`)))
  (`/Engine/EditorBlueprintResources/StandardMacros.IsValid` (`self.RelatedActor`)
    (:`Is Valid`
      (`/Engine/EditorBlueprintResources/StandardMacros.IsValid` (`self.OwnerPC`)
        (:`Is Valid`
          (bind _rotation (message `/Game/MapEditorExample/Blueprints/Pawns/I_Pawn.GetViewRotation` _returnvalue))
          (bind _location (message `/Game/MapEditorExample/Blueprints/Pawns/I_Pawn.GetViewLocation` _returnvalue))
          (set `self.OwnerLocation` _location)
          (set `self.OwnerRotation` _rotation))))))

(fn `InitializeForActor`
  (params (Actor :type "Actor Object Reference"))
  (returns (Button :type "UserWidget Object Reference"))
  (bind _output_get (set `self.RelatedActor` Actor))
  (`self.K2_SetActorLocation` (`self.K2_GetActorLocation` _output_get))
  (return (`self.PrimaryWidget`)))

(fn `UserConstructionScript`)